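; BP_End_Trigger is a level-end trigger that shows the win screen when the player reaches it.
; When the first player's pawn begins overlapping the Trigger component, the actor destroys itself and adds a BP_Win widget to the viewport.
; It then switches the player controller to UI-only input without mouse lock and shows the cursor.
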(event `self.Trigger.OnComponentBeginOverlap`
  (params (OverlappedComponent :type "PrimitiveComponent Object Reference") (OtherActor :type "Actor Object Reference") (OtherComp :type "PrimitiveComponent Object Reference") (OtherBodyIndex :type Integer) (bFromSweep :type Boolean) (SweepResult :type "HitResult Structure (by ref)"))
  (if (== OtherActor (`GameplayStatics.GetPlayerPawn` 0))
    (`self.K2_DestroyActor` (`ActorComponent.GetOwner` (`self.Trigger`)))
    (bind _returnvalue (`|CreateWidget` "/Game/Alessandro/UI/BP_Win.BP_Win_C"))
    (`UserWidget.AddToViewport` _returnvalue 0)
    (`WidgetBlueprintLibrary.SetInputMode_UIOnlyEx` (`GameplayStatics.GetPlayerController` 0) (`self.Win`))
    (bind _asplayer_controller (cast `PlayerController` (`GameplayStatics.GetPlayerController` 0)))
    (set `PlayerController.bShowMouseCursor` true _asplayer_controller)))

(fn `UserConstructionScript`)