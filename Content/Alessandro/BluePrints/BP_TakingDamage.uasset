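; BP_TakingDamage is a damageable pawn that loses Health on any damage and dies when it reaches zero or below.
; On death it unbinds the empty Dying event from OnTakeAnyDamage, destroys its capsule collision, plays a non-looping animation and detaches from its controller.
; The actor destroys itself after a short delay.
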(event `Dying` :!signature `self.OnTakeAnyDamage`
  (params (DamagedActor :type "Actor Object Reference") (Damage :type "Float (double-precision)") (DamageType :type "DamageType Object Reference") (InstigatedBy :type "Controller Object Reference") (DamageCauser :type "Actor Object Reference")))

(event `self.ReceiveAnyDamage`
  (params (Damage :type "Float (single-precision)") (DamageType :type "DamageType Object Reference") (InstigatedBy :type "Controller Object Reference") (DamageCauser :type "Actor Object Reference"))
  (bind _output_get (set `self.Health` (- (`self.Health`) Damage)))
  (if (<= _output_get 0.0)
    (remove `self.OnTakeAnyDamage` self (delegate `Dying`))
    (`ActorComponent.K2_DestroyComponent` (`self.Capsule (Collision Component)`))
    (`SkeletalMeshComponent.PlayAnimation` (`self.SkeletalMesh`) null false)
    (`self.DetachFromControllerPendingDestroy` self)
    (`KismetSystemLibrary.Delay` 3.0)
    (`self.K2_DestroyActor` self)))

(fn `UserConstructionScript`)