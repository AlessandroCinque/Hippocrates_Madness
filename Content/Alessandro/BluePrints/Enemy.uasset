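; Enemy AI character that chases the player, takes projectile damage and respawns on death.
; Pawn sensing feeds sightings to AIC_Enemy's blackboard and, within attack range, directly damages FirstPersonCharacter and plays an attack animation.
; Projectile hits on the capsule lower Health, shown through a widget health bar.
; At zero Health, Tick destroys it after a delay and is wired to spawn a replacement at a fixed location.
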(event `self.ReceiveTick`
  (params (DeltaSeconds :type "Float (single-precision)"))
  ;[1 1 1] Respawn
  (if (<= (`self.Health`) 0.0)
    (`/Engine/EditorBlueprintResources/StandardMacros.DoOnce` false
      (:`Completed`
        (`KismetSystemLibrary.Delay` 2.042)
        (`self.K2_DestroyActor`)
        (`AIBlueprintHelperLibrary.SpawnAIFromClass` "Enemy_C" "/Game/Adrian/AI/BT_Enemy.BT_Enemy" (178.0 130.0 245.0) (struct :`Yaw` 180.0))))))

(event `self.ReceiveBeginPlay`
  ;[1 1 1] Health Bar
  (bind _asbp_enem_hp_bar (cast `/Game/Alessandro/BluePrints/BP_Enem_HP_Bar` (`WidgetComponent.GetUserWidgetObject` (`self.Widget`))))
  (set `/Game/Alessandro/BluePrints/BP_Enem_HP_Bar.Owner` self _asbp_enem_hp_bar))

(event `self.CapsuleComponent.OnComponentHit`
  (params (HitComponent :type "PrimitiveComponent Object Reference") (OtherActor :type "Actor Object Reference") (OtherComp :type "PrimitiveComponent Object Reference") (NormalImpulse :type "Vector Structure") (Hit :type "HitResult Structure (by ref)"))
  ;[1 1 1] Enemy getting shoot
  (cast `/Game/FirstPersonCPP/Blueprints/FirstPersonProjectile` OtherActor)
  (set `self.Health` (- (`self.Health`) 10.0)))

(event `self.PawnSensing.OnSeePawn`
  (params (Pawn :type "Pawn Object Reference"))
  ;[1 1 1] Chasing Until Death
  (bind _output_get (set `self.Percieved Pawn` Pawn))
  (set `self.Player Location` (`self.K2_GetActorLocation` _output_get))
  (bind _asaic_enemy (cast `/Game/Adrian/AI/AIC_Enemy` (`AIBlueprintHelperLibrary.GetAIController` self)))
  (bind _output_get_2 (set `self.AI Controller` _asaic_enemy))
  (`/Game/Adrian/AI/AIC_Enemy.UpdateHasLineOfSight` _output_get_2 true)
  (`/Game/Adrian/AI/AIC_Enemy.UpdatePlayerActorKey` (`self.AI Controller`) (`self.Percieved Pawn`))
  (if (<= (`self.Health`) 0.0)
    (`self.DetachFromControllerPendingDestroy` self)
    (else
      ;[1 1 1] Attacking the Player
      (if (<= (`KismetMathLibrary.Vector_Distance` (`self.K2_GetActorLocation` self) (`self.Player Location`)) (`self.Attack Range`))
        (bind _asfirst_person_character (cast `/Game/FirstPersonCPP/Blueprints/FirstPersonCharacter` (`self.Percieved Pawn`)))
        (set `/Game/FirstPersonCPP/Blueprints/FirstPersonCharacter.FullHealth` (- (`/Game/FirstPersonCPP/Blueprints/FirstPersonCharacter.FullHealth` _asfirst_person_character) (`self.Damage`)) _asfirst_person_character)
        (`SkeletalMeshComponent.PlayAnimation` (`self.Mesh`) "/Game/Alessandro/Artists_Stuff/Dora/Character/Little_Fucker/Attack/Attack.Attack" false)))))

(fn `UpdateWalkSpeed`
  (params (NewSpeed :type "Float (double-precision)"))
  (set `CharacterMovementComponent.MaxWalkSpeed` NewSpeed (`self.CharacterMovement`)))

(fn `UserConstructionScript`)