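; BP_Spawn_1 is an enemy spawner that creates Enemy AI pawns at its PortalBox location.
; Easy, Medium and Hard events serve as difficulty levels, each allowing a higher cap on live enemies.
; Each call counts all Enemy actors in the world and spawns one more only while under that cap.
; Nothing in this Blueprint calls these events, as BeginPlay, overlap and Tick are disabled.
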(event `Easy`
  ;[1 1 1] Level 1
  (bind _outactors (`GameplayStatics.GetAllActorsOfClass` "/Game/Alessandro/BluePrints/Enemy.Enemy_C"))
  (if (< (`KismetArrayLibrary.Array_Length` _outactors) 5)
    (`AIBlueprintHelperLibrary.SpawnAIFromClass` "/Game/Alessandro/BluePrints/Enemy.Enemy_C" null (`SceneComponent.K2_GetComponentLocation` (`self.Portal_box`)))))

(event `Medium`
  ;[1 1 1] Level 2
  (bind _outactors (`GameplayStatics.GetAllActorsOfClass` "/Game/Alessandro/BluePrints/Enemy.Enemy_C"))
  (if (< (`KismetArrayLibrary.Array_Length` _outactors) 10)
    (`AIBlueprintHelperLibrary.SpawnAIFromClass` "/Game/Alessandro/BluePrints/Enemy.Enemy_C" null (`SceneComponent.K2_GetComponentLocation` (`self.Portal_box`)))))

(event `Hard`
  ;[1 1 1] Level 3
  (bind _outactors (`GameplayStatics.GetAllActorsOfClass` "/Game/Alessandro/BluePrints/Enemy.Enemy_C"))
  (if (< (`KismetArrayLibrary.Array_Length` _outactors) 15)
    (`AIBlueprintHelperLibrary.SpawnAIFromClass` "/Game/Alessandro/BluePrints/Enemy.Enemy_C" null (`SceneComponent.K2_GetComponentLocation` (`self.Portal_box`)))))

(fn `UserConstructionScript`)